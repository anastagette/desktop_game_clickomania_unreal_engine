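; Demo-style cube actor that spins continuously and responds to mouse clicks.
; Tick adds frame-rate independent world roll from a speed variable, while each click adds a fixed local rotation step.
; BeginPlay and clicks call ToggleColor, which swaps the cube's material between Oyster and Tan via a boolean flag.
; A Move helper for local offsets exists, but its only call is never executed.
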(event `self.ReceiveTick`
  (params (DeltaSeconds :type "Float (single-precision)"))
  (`self.K2_AddActorWorldRotation` (`KismetMathLibrary.MakeRotator` (* DeltaSeconds (`self.RollSpeecd`)))))

(event `self.ReceiveActorOnClicked`
  (params (ButtonPressed :type "Key Structure"))
  (`self.K2_AddActorLocalRotation` (struct :`Yaw` 30.0))
  (`self.ToggleColor`))

(event `self.ReceiveBeginPlay`
  (`self.ToggleColor`))

(fn `Move`
  (params (Offset :type "Vector Structure"))
  (returns (Success :type Boolean))
  (`self.K2_AddActorLocalOffset` Offset)
  (return true))

(fn `ToggleColor`
  (bind _cube (`self.Cube`))
  (if (`self.IsGreen`)
    (`PrimitiveComponent.SetMaterial` _cube 0 "/Game/Materials/Oyster.Oyster")
    (else
      (`PrimitiveComponent.SetMaterial` _cube 0 "/Game/Materials/Tan.Tan")))
  (set `self.IsGreen` (not (`self.IsGreen`))))

(fn `UserConstructionScript`)