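; Clickable Item actor for a field-based game, showing a colored cube.
; On BeginPlay, the Color value selects a green, yellow or pink material for the cube.
; Clicks are forwarded to the Field through OnItemClick, and a MoveTo event slides the item's root to a given relative location with an eased one-second move.
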(event `self.ReceiveBeginPlay`
  (bind _cube (`self.Cube`))
  (switch `int` (`self.Color`)
    (:`0`
      (`PrimitiveComponent.SetMaterial` _cube 0 "/Game/Materials/Green.Green"))
    (:`1`
      (`PrimitiveComponent.SetMaterial` _cube 0 "/Game/Materials/Yellow.Yellow"))
    (:`2`
      (`PrimitiveComponent.SetMaterial` _cube 0 "/Game/Materials/Pink.Pink"))))

(event `self.ReceiveActorOnClicked`
  (params (ButtonPressed :type "Key Structure"))
  (`/Game/Blueprints/Field.OnItemClick` (`self.Field`) self))

(event `MoveTo`
  (params (Location :type "Vector Structure"))
  (`KismetSystemLibrary.MoveComponentTo` (`self.DefaultSceneRoot`) Location (struct) true true 1.0))

(fn `UserConstructionScript`)